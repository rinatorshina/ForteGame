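; Tabbie, a cat NPC who gives quest dialogue about a broken tambourine and a feud with Penny when the player interacts.
; Interaction picks one of four dialogue functions from Teddy's quest completion, its own SpokenTo flag and Penny's SpokeWith flag.
; Each function starts the talking animation, hides the player prompt and shows a typewriter dialogue widget.
; The event polls each tick until typing finishes, then restores idle and sets SpokenTo or BunbunMentioned where relevant.
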(event EventBeginPlay
  (bind _outactors (Actor|GetAllActorsOfClass "/Game/Blueprints/StateSwitchManager.StateSwitchManager_C"))
  (bind _asbp_first_person_character (Utilities|Casting|CastToBP_FirstPersonCharacter (Game|Player|GetPlayerPawn 0)))
  (Variables|Default|SetPlayer _asbp_first_person_character))

(event EventOnInteractedwith
  (bind _outactors (Actor|GetAllActorsOfClass "/Game/Blueprints/TeddyBP.TeddyBP_C"))
  (if (Variables|/Game/Blueprints/TeddyBP.TeddyBP_C|GetTeddyQuestCompleted (Utilities|Array|Get(acopy) _outactors))
    (if (Variables|Default|GetSpokenTo)
      (bind _outactors_2 (Actor|GetAllActorsOfClass "/Game/Blueprints/PennyBP.PennyBP_C"))
      (if (Variables|/Game/Blueprints/PennyBP.PennyBP_C|GetSpokeWith (Utilities|Array|Get(acopy) _outactors_2))
        (bind _dialogue_box (CallFunction|IdleAfterPenny))
        (if (Variables|/Game/Blueprints/Widgets/DialogueBoxWBP.DialogueBoxWBP_C|GetTypewriterFinished _dialogue_box) :!label _label
          (Components|Animation|PlayAnimation (Variables|Default|GetTabbie_tp_fixed) "/Game/Assets/Animations/TabbieFix_Anim/Idle.Idle" true)
          (Variables|Default|SetBunbunMentioned true)
          (else
            (Utilities|FlowControl|DelayUntilNextTick)
            (goto _label)))
        (else
          (bind _dialogue_box_2 (CallFunction|IdleBeforePenny))
          (if (Variables|/Game/Blueprints/Widgets/DialogueBoxWBP.DialogueBoxWBP_C|GetTypewriterFinished _dialogue_box_2) :!label _label_2
            (Components|Animation|PlayAnimation (Variables|Default|GetTabbie_tp_fixed) "/Game/Assets/Animations/TabbieFix_Anim/Idle.Idle" true)
            (else
              (Utilities|FlowControl|DelayUntilNextTick)
              (goto _label_2)))))
      (else
        (bind _dialogue_box_3 (CallFunction|OpeningDialogue))
        (if (Variables|/Game/Blueprints/Widgets/DialogueBoxWBP.DialogueBoxWBP_C|GetTypewriterFinished _dialogue_box_3) :!label _label_3
          (Components|Animation|PlayAnimation (Variables|Default|GetTabbie_tp_fixed) "/Game/Assets/Animations/TabbieFix_Anim/Idle.Idle" true)
          (Variables|Default|SetSpokenTo true)
          (else
            (Utilities|FlowControl|DelayUntilNextTick)
            (goto _label_3)))))
    (else
      (bind _dialogue_box_4 (CallFunction|BlankIdle))
      (if (Variables|/Game/Blueprints/Widgets/DialogueBoxWBP.DialogueBoxWBP_C|GetTypewriterFinished _dialogue_box_4) :!label _label_4
        (Components|Animation|PlayAnimation (Variables|Default|GetTabbie_tp_fixed) "/Game/Assets/Animations/TabbieFix_Anim/Idle.Idle" true)
        (else
          (Utilities|FlowControl|DelayUntilNextTick)
          (goto _label_4))))))

(fn ConstructionScript
  (|CallParentFunction))

(fn OpeningDialogue
  (Components|Animation|PlayAnimation (Variables|Default|GetTabbie_tp_fixed) "/Game/Assets/Animations/TabbieFix_Anim/Talking.Talking" true)
  (Default|HidePrompt (Variables|Default|GetPlayer))
  (bind _returnvalue (UserInterface|CreateWidget "/Game/Blueprints/Widgets/DialogueDisplayWBP.DialogueDisplayWBP_C"))
  (UserInterface|Viewport|AddtoViewport _returnvalue 0)
  (bind _returnvalue_2 (UserInterface|CreateWidget "/Game/Blueprints/Widgets/DialogueBoxWBP.DialogueBoxWBP_C" 0 (Utilities|Array|MakeArray "Answer me this, Sammy: how's a cat s'pposed to groove, s'pposed to beat, s'pposed to bop... with a tambourine with no cymbals?!" "I'm tearing my fur out here!!! Don't believe whatever that penickety penguin tells you!" "I DID NOT TAKE HER BUTTON!!!") 3.5))
  (Default|AddWidgettoStack _returnvalue _returnvalue_2)
  (return _returnvalue_2))

(fn BlankIdle
  (Components|Animation|PlayAnimation (Variables|Default|GetTabbie_tp_fixed) "/Game/Assets/Animations/TabbieFix_Anim/Talking.Talking" true)
  (Default|HidePrompt (Variables|Default|GetPlayer))
  (bind _returnvalue (UserInterface|CreateWidget "/Game/Blueprints/Widgets/DialogueDisplayWBP.DialogueDisplayWBP_C"))
  (UserInterface|Viewport|AddtoViewport _returnvalue 0)
  (bind _returnvalue_2 (UserInterface|CreateWidget "/Game/Blueprints/Widgets/DialogueBoxWBP.DialogueBoxWBP_C" 0 (Utilities|Array|MakeArray "Ah, Sammy! I could really use your help here, but I think Teddy has something to talk to you about first...") 3.5))
  (Default|AddWidgettoStack _returnvalue _returnvalue_2)
  (return _returnvalue_2))

(fn IdleBeforePenny
  (Components|Animation|PlayAnimation (Variables|Default|GetTabbie_tp_fixed) "/Game/Assets/Animations/TabbieFix_Anim/Talking.Talking" true)
  (Default|HidePrompt (Variables|Default|GetPlayer))
  (bind _returnvalue (UserInterface|CreateWidget "/Game/Blueprints/Widgets/DialogueDisplayWBP.DialogueDisplayWBP_C"))
  (UserInterface|Viewport|AddtoViewport _returnvalue 0)
  (bind _returnvalue_2 (UserInterface|CreateWidget "/Game/Blueprints/Widgets/DialogueBoxWBP.DialogueBoxWBP_C" 0 (Utilities|Array|MakeArray "Button this, button that! But what about MY tambourine?!") 3.5))
  (Default|AddWidgettoStack _returnvalue _returnvalue_2)
  (return _returnvalue_2))

(fn IdleAfterPenny
  (Components|Animation|PlayAnimation (Variables|Default|GetTabbie_tp_fixed) "/Game/Assets/Animations/TabbieFix_Anim/Talking.Talking" true)
  (Default|HidePrompt (Variables|Default|GetPlayer))
  (bind _returnvalue (UserInterface|CreateWidget "/Game/Blueprints/Widgets/DialogueDisplayWBP.DialogueDisplayWBP_C"))
  (UserInterface|Viewport|AddtoViewport _returnvalue 0)
  (bind _returnvalue_2 (UserInterface|CreateWidget "/Game/Blueprints/Widgets/DialogueBoxWBP.DialogueBoxWBP_C" 0 (Utilities|Array|MakeArray "She's making the fort frosty! She's upsetting poor Bunbun!" "I saw him whispering into his trumpet earlier - all this shouting is making his stitching come loose!") 3.5))
  (Default|AddWidgettoStack _returnvalue _returnvalue_2)
  (return _returnvalue_2))