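; TrumpetBP is an interactable trumpet that hides a button component named AccordionButton, used in solving a quest.
; The button is hidden at BeginPlay, and interaction has no effect unless SolutionAvailable is set on the first BunbunBP in the level.
; The first valid interaction reveals the button and sets ButtonFound.
; Later valid interactions call QuestSolved on the first SolutionSceneBP found.
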(event EventBeginPlay
  ;[0.15 0.15 0.15 0.5] Makes button invisible
  (Rendering|SetVisibility (Variables|Default|GetAccordion_button) false false))

(event EventOnInteractedwith
  (bind _outactors (Actor|GetAllActorsOfClass "/Game/Blueprints/BunbunBP.BunbunBP_C"))
  (if (Variables|/Game/Blueprints/BunbunBP.BunbunBP_C|GetSolutionAvailable (Utilities|Array|Get(acopy) _outactors))
    (if (Variables|Default|GetButtonFound)
      (bind _outactors_2 (Actor|GetAllActorsOfClass "/Game/Blueprints/SolutionSceneBP.SolutionSceneBP_C"))
      (Default|QuestSolved (Utilities|Array|Get(acopy) _outactors_2))
      (else
        (Rendering|SetVisibility (Variables|Default|GetAccordion_button) true false)
        (Variables|Default|SetButtonFound true)))))

(fn ConstructionScript
  (|CallParentFunction))