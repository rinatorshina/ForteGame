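; Star prop that switches between a paper look with a visible string in the real state and a glowing look in the dream state.
; BeginPlay hides the string and creates a dynamic material instance on the cube.
; RealStars and DreamStars set the material parameter, point light intensity and string visibility.
; OnTransitionProgress scales the parameter with progress, while its zero-alpha Lerp passes raw progress as light intensity.
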(event Custom|RealStars
  ;[0.15 0.15 0.15 0.5] State Related Events
  (CallFunction|PaperStars))

(event Custom|DreamStars
  ;[0.15 0.15 0.15 0.5] State Related Events
  (CallFunction|GlowingStars))

(event Custom|OnTransitionProgress
  (params (Progress :type Float%20%28double-precision%29))
  (Rendering|Material|SetScalarParameterValue (Variables|Default|GetStarsMaterial) "Param" (* Progress 3.0) :!class /Script/Engine.MaterialInstanceDynamic)
  (Rendering|Components|Light|SetIntensity (Variables|Default|GetPointLight) (Math|Float|Lerp Progress 15.0 0.0)))

(event EventBeginPlay
  (Rendering|SetVisibility (Variables|Default|GetString) false false)
  (bind _returnvalue (Rendering|Material|CreateDynamicMaterialInstance (Variables|Default|GetCube) 0 "/Game/Assets/Props/PaperStarMaterial.PaperStarMaterial" "None" :!class /Script/Engine.PrimitiveComponent))
  (bind _output_get (Variables|Default|SetStarsMaterial _returnvalue))
  (Rendering|Material|SetScalarParameterValue _output_get "Param" 5.0 :!class /Script/Engine.MaterialInstanceDynamic))

(fn ConstructionScript)

(fn PaperStars
  (Rendering|Material|SetScalarParameterValue (Variables|Default|GetStarsMaterial) "Param" 0.0 :!class /Script/Engine.MaterialInstanceDynamic)
  (Rendering|Components|Light|SetIntensity (Variables|Default|GetPointLight) 0.0)
  (Rendering|SetVisibility (Variables|Default|GetString) true false))

(fn GlowingStars
  (Rendering|Material|SetScalarParameterValue (Variables|Default|GetStarsMaterial) "Param" 3.0 :!class /Script/Engine.MaterialInstanceDynamic)
  (Rendering|Components|Light|SetIntensity (Variables|Default|GetPointLight) 4.0)
  (Rendering|SetVisibility (Variables|Default|GetString) false false))