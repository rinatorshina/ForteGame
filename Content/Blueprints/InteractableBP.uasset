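; InteractableBP is an interactable actor that tracks whether it is being looked at and can travel along a spline route.
; GazedAt and NoGaze toggle a LookedAt flag, while OnInteractedWith is an empty event.
; StartRunning plays a timeline that maps progress to distance along RouteSpline's spline and sets the actor's world location each update.
; BeginPlay stores the start location.
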(event Custom|GazedAt
  ;[0.15 0.15 0.15 0.5] Detect if being looked at
  (Variables|Default|SetLookedAt true))

(event Custom|StartRunning
  (bind _routespline (Variables|Default|GetRouteSpline))
  (bind _spline (Variables|/Game/Blueprints/RouteSplineBP.RouteSplineBP_C|GetSpline _routespline))
  (bind _progress (Timeline|MoveTimeline Play)
    (:Update
      (bind _output_get (Variables|Default|SetSplineLength1 (Spline|GetSplineLength _spline)))
      (Transformation|SetActorLocation (Spline|GetLocationatDistanceAlongSpline _spline (* _progress _output_get) "World") false false))))

(event Custom|NoGaze
  ;[0.15 0.15 0.15 0.5] Detect if being looked at
  (Variables|Default|SetLookedAt false))

(event Custom|OnInteractedWith)

(event EventBeginPlay
  (Variables|Default|SetStartLocation (Transformation|GetActorLocation)))

(fn ConstructionScript)