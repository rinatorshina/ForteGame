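; Quest NPC Penny, who tells Sammy about her stolen accordion button and feud with Tabbie.
; On interaction, StateSwitchManager's state selects either dialogue or a focus hint, with lines gated by Teddy's quest, SpokeWith and Tabbie's SpokenTo.
; Helper functions spawn typewriter widgets and start the talking animation, while the event graph polls each tick for completion.
; After the post-Tabbie line, it calls SwitchState while TriggerCount is below its threshold, otherwise returning to idle.
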(event EventBeginPlay
  (bind _outactors (Actor|GetAllActorsOfClass "/Game/Blueprints/StateSwitchManager.StateSwitchManager_C"))
  (bind _asbp_first_person_character (Utilities|Casting|CastToBP_FirstPersonCharacter (Game|Player|GetPlayerPawn 0)))
  (Variables|Default|SetPlayer _asbp_first_person_character))

(event EventOnInteractedwith
  (if (Utilities|Enum|Equal(Enum) (Variables|/Game/Blueprints/StateSwitchManager.StateSwitchManager_C|GetCurrentState (Utilities|Array|Get(acopy) (stale EventBeginPlay _outactors))) "NewEnumerator0")
    (bind _outactors (Actor|GetAllActorsOfClass "/Game/Blueprints/TeddyBP.TeddyBP_C"))
    (if (Variables|/Game/Blueprints/TeddyBP.TeddyBP_C|GetTeddyQuestCompleted (Utilities|Array|Get(acopy) _outactors))
      (if (Variables|Default|GetSpokeWith)
        (bind _outactors_2 (Actor|GetAllActorsOfClass "/Game/Blueprints/TabbieBP.TabbieBP_C"))
        (if (Variables|/Game/Blueprints/TabbieBP.TabbieBP_C|GetSpokenTo (Utilities|Array|Get(acopy) _outactors_2))
          (bind _dialogue_box (CallFunction|IdleAfterTabbie))
          (if (Variables|/Game/Blueprints/Widgets/DialogueBoxWBP.DialogueBoxWBP_C|GetTypewriterFinished _dialogue_box) :!label _label
            (if (>= (Variables|/Game/Blueprints/StateSwitchManager.StateSwitchManager_C|GetTriggerCount (Utilities|Array|Get(acopy) (stale EventBeginPlay _outactors))) 4)
              (Components|Animation|PlayAnimation (Variables|Default|GetT-Pose) "/Game/Assets/Animations/Penny_anims/Idle.Idle" true)
              (else
                (Default|SwitchState (Utilities|Array|Get(acopy) (stale EventBeginPlay _outactors)))))
            (else
              (Utilities|FlowControl|DelayUntilNextTick)
              (goto _label)))
          (else
            (bind _dialogue_box_2 (CallFunction|IdleBeforeTabbie))
            (if (Variables|/Game/Blueprints/Widgets/DialogueBoxWBP.DialogueBoxWBP_C|GetTypewriterFinished _dialogue_box_2) :!label _label_2
              (Components|Animation|PlayAnimation (Variables|Default|GetT-Pose) "/Game/Assets/Animations/Penny_anims/Idle.Idle" true)
              (else
                (Utilities|FlowControl|DelayUntilNextTick)
                (goto _label_2)))))
        (else
          (bind _dialogue_box_3 (CallFunction|OpeningDialogue))
          (if (Variables|/Game/Blueprints/Widgets/DialogueBoxWBP.DialogueBoxWBP_C|GetTypewriterFinished _dialogue_box_3) :!label _label_3
            (Components|Animation|PlayAnimation (Variables|Default|GetT-Pose) "/Game/Assets/Animations/Penny_anims/Idle.Idle" true)
            (bind _dialogue_box_4 (CallFunction|OpeningDialogue2))
            (if (Variables|/Game/Blueprints/Widgets/DialogueBoxWBP.DialogueBoxWBP_C|GetTypewriterFinished _dialogue_box_4) :!label _label_4
              (Components|Animation|PlayAnimation (Variables|Default|GetT-Pose) "/Game/Assets/Animations/Penny_anims/Idle.Idle" true)
              (bind _dialogue_box_5 (CallFunction|OpeningDialogue3))
              (if (Variables|/Game/Blueprints/Widgets/DialogueBoxWBP.DialogueBoxWBP_C|GetTypewriterFinished _dialogue_box_5) :!label _label_5
                (Components|Animation|PlayAnimation (Variables|Default|GetT-Pose) "/Game/Assets/Animations/Penny_anims/Idle.Idle" true)
                (Variables|Default|SetSpokeWith true)
                (else
                  (Utilities|FlowControl|DelayUntilNextTick)
                  (goto _label_5)))
              (else
                (Utilities|FlowControl|DelayUntilNextTick)
                (goto _label_4)))
            (else
              (Utilities|FlowControl|DelayUntilNextTick)
              (goto _label_3)))))
      (else
        (bind _dialogue_box_6 (CallFunction|BlankIdle))
        (if (Variables|/Game/Blueprints/Widgets/DialogueBoxWBP.DialogueBoxWBP_C|GetTypewriterFinished _dialogue_box_6) :!label _label_6
          (Components|Animation|PlayAnimation (Variables|Default|GetT-Pose) "/Game/Assets/Animations/Penny_anims/Idle.Idle" true)
          (else
            (Utilities|FlowControl|DelayUntilNextTick)
            (goto _label_6)))))
    (else
      (CallFunction|RealityState))))

(fn ConstructionScript
  (|CallParentFunction))

(fn OpeningDialogue
  (Components|Animation|PlayAnimation (Variables|Default|GetT-Pose) "/Game/Assets/Animations/Penny_anims/Talking.Talking" true)
  (Default|HidePrompt (Variables|Default|GetPlayer))
  (bind _returnvalue (UserInterface|CreateWidget "/Game/Blueprints/Widgets/DialogueDisplayWBP.DialogueDisplayWBP_C"))
  (UserInterface|Viewport|AddtoViewport _returnvalue 0)
  (bind _returnvalue_2 (UserInterface|CreateWidget "/Game/Blueprints/Widgets/DialogueBoxWBP.DialogueBoxWBP_C" 0 (Utilities|Array|MakeArray "Oh, Sammy! It's all too terrible! My dreams! Turned to dust!" "This concert was supposed to be MY big moment. For once, a chance for ME to be a STAR! But!" "SABOTAGE!") 3.5))
  (Default|AddWidgettoStack _returnvalue _returnvalue_2)
  (return _returnvalue_2))

(fn OpeningDialogue2
  (Components|Animation|PlayAnimation (Variables|Default|GetT-Pose) "/Game/Assets/Animations/Penny_anims/Talking.Talking" true)
  (Default|HidePrompt (Variables|Default|GetPlayer))
  (bind _returnvalue (UserInterface|CreateWidget "/Game/Blueprints/Widgets/DialogueDisplayWBP.DialogueDisplayWBP_C"))
  (UserInterface|Viewport|AddtoViewport _returnvalue 0)
  (bind _returnvalue_2 (UserInterface|CreateWidget "/Game/Blueprints/Widgets/DialogueBoxWBP.DialogueBoxWBP_C" 0 (Utilities|Array|MakeArray "The button fell off of my beloved accordion while I was practicing this morning and before I could fix it..." "SOMEBODY stole it! I'm not usually one to point flippers, but... I'm certain of who did it.") 3.5))
  (Default|AddWidgettoStack _returnvalue _returnvalue_2)
  (return _returnvalue_2))

(fn OpeningDialogue3
  (Components|Animation|PlayAnimation (Variables|Default|GetT-Pose) "/Game/Assets/Animations/Penny_anims/Talking.Talking" true)
  (Default|HidePrompt (Variables|Default|GetPlayer))
  (bind _returnvalue (UserInterface|CreateWidget "/Game/Blueprints/Widgets/DialogueDisplayWBP.DialogueDisplayWBP_C"))
  (UserInterface|Viewport|AddtoViewport _returnvalue 0)
  (bind _returnvalue_2 (UserInterface|CreateWidget "/Game/Blueprints/Widgets/DialogueBoxWBP.DialogueBoxWBP_C" 0 (Utilities|Array|MakeArray "Let's just say, she doesn't have a helpful heart and a patient paw - more like wicked whiskers and a thieving claw!" "So I've taken something of hers... and I WON'T be returning it until that feline frenemy gives back what's MINE!" "Please get it back, Sammy! You'll know it when you see it - it looks like a little penny. Oh... Hah! Get it? Penny!") 3.5))
  (Default|AddWidgettoStack _returnvalue _returnvalue_2)
  (return _returnvalue_2))

(fn IdleBeforeTabbie
  (Components|Animation|PlayAnimation (Variables|Default|GetT-Pose) "/Game/Assets/Animations/Penny_anims/Talking.Talking" true)
  (Default|HidePrompt (Variables|Default|GetPlayer))
  (bind _returnvalue (UserInterface|CreateWidget "/Game/Blueprints/Widgets/DialogueDisplayWBP.DialogueDisplayWBP_C"))
  (UserInterface|Viewport|AddtoViewport _returnvalue 0)
  (bind _returnvalue_2 (UserInterface|CreateWidget "/Game/Blueprints/Widgets/DialogueBoxWBP.DialogueBoxWBP_C" 0 (Utilities|Array|MakeArray "An eye for an eye! A beak for a beak! I want MY button... beek.") 3.5))
  (Default|AddWidgettoStack _returnvalue _returnvalue_2)
  (return _returnvalue_2))

(fn BlankIdle
  (Components|Animation|PlayAnimation (Variables|Default|GetT-Pose) "/Game/Assets/Animations/Penny_anims/Talking.Talking" true)
  (Default|HidePrompt (Variables|Default|GetPlayer))
  (bind _returnvalue (UserInterface|CreateWidget "/Game/Blueprints/Widgets/DialogueDisplayWBP.DialogueDisplayWBP_C"))
  (UserInterface|Viewport|AddtoViewport _returnvalue 0)
  (bind _returnvalue_2 (UserInterface|CreateWidget "/Game/Blueprints/Widgets/DialogueBoxWBP.DialogueBoxWBP_C" 0 (Utilities|Array|MakeArray "Oh, hey, Sammy. I think Teddy wants to talk to you...") 3.5))
  (Default|AddWidgettoStack _returnvalue _returnvalue_2)
  (return _returnvalue_2))

(fn IdleAfterTabbie
  (Components|Animation|PlayAnimation (Variables|Default|GetT-Pose) "/Game/Assets/Animations/Penny_anims/Talking.Talking" true)
  (Default|HidePrompt (Variables|Default|GetPlayer))
  (bind _returnvalue (UserInterface|CreateWidget "/Game/Blueprints/Widgets/DialogueDisplayWBP.DialogueDisplayWBP_C"))
  (UserInterface|Viewport|AddtoViewport _returnvalue 0)
  (bind _returnvalue_2 (UserInterface|CreateWidget "/Game/Blueprints/Widgets/DialogueBoxWBP.DialogueBoxWBP_C" 0 (Utilities|Array|MakeArray "That cantankerous cat STILL denies it?! If SHE doesn't have my button, who DOES?") 3.5))
  (Default|AddWidgettoStack _returnvalue _returnvalue_2)
  (return _returnvalue_2))

(fn RealityState
  (Default|HidePrompt (Variables|Default|GetPlayer))
  (bind _returnvalue (UserInterface|CreateWidget "/Game/Blueprints/Widgets/DialogueDisplayWBP.DialogueDisplayWBP_C"))
  (UserInterface|Viewport|AddtoViewport _returnvalue 0)
  (bind _returnvalue_2 (UserInterface|CreateWidget "/Game/Blueprints/Widgets/DialogueBoxWBP.DialogueBoxWBP_C" 0 (Utilities|Array|MakeArray "Focus by holding down [Space Bar]") 3.0))
  (Default|AddWidgettoStack _returnvalue _returnvalue_2)
  (return _returnvalue_2))