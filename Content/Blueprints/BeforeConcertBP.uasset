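; Scripts the pre-concert toy sequence, started by the TimeToChoose event.
; Teddy claps through a typewriter congratulation, then Penny, Tabbie, Bunbun and Teddy walk as Toy-tagged interactables start running.
; After a delay they switch to music or idle animations, and Teddy's count-in line ends by calling SwitchState on the StateSwitchManager.
; Each dialogue line returns its widget, which the event polls every tick until typing finishes.
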(event Custom|TimeToChoose
  (bind _dialogue_box (CallFunction|TeddyLine1))
  (if (Variables|/Game/Blueprints/Widgets/DialogueBoxWBP.DialogueBoxWBP_C|GetTypewriterFinished _dialogue_box) :!label _label
    (CallFunction|BacktoIdle)
    (CallFunction|ToysRun)
    (Utilities|FlowControl|Delay 6.0)
    (CallFunction|MusicIdles)
    (bind _dialogue_box_2 (CallFunction|TeddyLine2))
    (if (Variables|/Game/Blueprints/Widgets/DialogueBoxWBP.DialogueBoxWBP_C|GetTypewriterFinished _dialogue_box_2) :!label _label_2
      (Default|SwitchState (Utilities|Array|Get(acopy) (stale EventBeginPlay _outactors)))
      (else
        (Utilities|FlowControl|DelayUntilNextTick)
        (goto _label_2)))
    (else
      (Utilities|FlowControl|DelayUntilNextTick)
      (goto _label))))

(event EventBeginPlay
  (bind _outactors (Actor|GetAllActorsOfClass "/Game/Blueprints/StateSwitchManager.StateSwitchManager_C"))
  (bind _asbp_first_person_character (Utilities|Casting|CastToBP_FirstPersonCharacter (Game|Player|GetPlayerPawn 0)))
  (Variables|Default|SetPlayer _asbp_first_person_character))

(fn ConstructionScript)

(fn TeddyLine1
  (bind _outactors (Actor|GetAllActorsOfClass "/Game/Blueprints/TeddyBP.TeddyBP_C"))
  (Components|Animation|PlayAnimation (Variables|/Game/Blueprints/TeddyBP.TeddyBP_C|GetT_Pose (Utilities|Array|Get(acopy) _outactors)) "/Game/Assets/Animations/Teddy_Anima/Clapping.Clapping" false)
  (Default|HidePrompt (Variables|Default|GetPlayer))
  (bind _returnvalue (UserInterface|CreateWidget "/Game/Blueprints/Widgets/DialogueDisplayWBP.DialogueDisplayWBP_C"))
  (UserInterface|Viewport|AddtoViewport _returnvalue 0)
  (bind _returnvalue_2 (UserInterface|CreateWidget "/Game/Blueprints/Widgets/DialogueBoxWBP.DialogueBoxWBP_C" 0 (Utilities|Array|MakeArray "You did it! Remember, Sammio, you can solve any problem with a helpful heart and a patient paw!") 4.0))
  (Default|AddWidgettoStack _returnvalue _returnvalue_2)
  (return _returnvalue_2))

(fn ToysRun
  (bind _outactors (Actor|GetAllActorsOfClass "/Game/Blueprints/PennyBP.PennyBP_C"))
  (Components|Animation|PlayAnimation (Variables|/Game/Blueprints/PennyBP.PennyBP_C|GetT-Pose (Utilities|Array|Get(acopy) _outactors)) "/Game/Assets/Animations/Penny_anims/Walking.Walking" true)
  (bind _outactors_2 (Actor|GetAllActorsOfClass "/Game/Blueprints/TabbieBP.TabbieBP_C"))
  (Components|Animation|PlayAnimation (Variables|/Game/Blueprints/TabbieBP.TabbieBP_C|GetTabbie_tp_fixed (Utilities|Array|Get(acopy) _outactors_2)) "/Game/Assets/Animations/TabbieFix_Anim/Walking.Walking" true)
  (bind _outactors_3 (Actor|GetAllActorsOfClass "/Game/Blueprints/BunbunBP.BunbunBP_C"))
  (Components|Animation|PlayAnimation (Variables|/Game/Blueprints/BunbunBP.BunbunBP_C|GetBunbun_tp_fixed (Utilities|Array|Get(acopy) _outactors_3)) "/Game/Assets/Animations/BunbunFix_Anim/Walking.Walking" true)
  (bind _outactors_4 (Actor|GetAllActorsOfClass "/Game/Blueprints/TeddyBP.TeddyBP_C"))
  (Components|Animation|PlayAnimation (Variables|/Game/Blueprints/TeddyBP.TeddyBP_C|GetT_Pose (Utilities|Array|Get(acopy) _outactors_4)) "/Game/Assets/Animations/Teddy_Anima/Walking.Walking" true)
  (bind _outactors_5 (Actor|GetAllActorsOfClasswithTag "/Game/Blueprints/InteractableBP.InteractableBP_C" "Toy"))
  (for _array_element _outactors_5
    (Default|StartRunning _array_element)))

(fn BacktoIdle
  (bind _outactors (Actor|GetAllActorsOfClass "/Game/Blueprints/PennyBP.PennyBP_C"))
  (Components|Animation|PlayAnimation (Variables|/Game/Blueprints/PennyBP.PennyBP_C|GetT-Pose (Utilities|Array|Get(acopy) _outactors)) "/Game/Assets/Animations/Penny_anims/Idle.Idle" true)
  (bind _outactors_2 (Actor|GetAllActorsOfClass "/Game/Blueprints/TabbieBP.TabbieBP_C"))
  (Components|Animation|PlayAnimation (Variables|/Game/Blueprints/TabbieBP.TabbieBP_C|GetTabbie_tp_fixed (Utilities|Array|Get(acopy) _outactors_2)) "/Game/Assets/Animations/TabbieFix_Anim/Idle.Idle" true)
  (bind _outactors_3 (Actor|GetAllActorsOfClass "/Game/Blueprints/BunbunBP.BunbunBP_C"))
  (Components|Animation|PlayAnimation (Variables|/Game/Blueprints/BunbunBP.BunbunBP_C|GetBunbun_tp_fixed (Utilities|Array|Get(acopy) _outactors_3)) "/Game/Assets/Animations/BunbunFix_Anim/Idle.Idle" true)
  (bind _outactors_4 (Actor|GetAllActorsOfClass "/Game/Blueprints/TeddyBP.TeddyBP_C"))
  (Components|Animation|PlayAnimation (Variables|/Game/Blueprints/TeddyBP.TeddyBP_C|GetT_Pose (Utilities|Array|Get(acopy) _outactors_4)) "/Game/Assets/Animations/Teddy_Anima/Idle.Idle" true))

(fn TeddyLine2
  (bind _outactors (Actor|GetAllActorsOfClass "/Game/Blueprints/TeddyBP.TeddyBP_C"))
  (Components|Animation|PlayAnimation (Variables|/Game/Blueprints/TeddyBP.TeddyBP_C|GetT_Pose (Utilities|Array|Get(acopy) _outactors)) "/Game/Assets/Animations/Teddy_Anima/Music_idle.Music_idle" true)
  (Default|HidePrompt (Variables|Default|GetPlayer))
  (bind _returnvalue (UserInterface|CreateWidget "/Game/Blueprints/Widgets/DialogueDisplayWBP.DialogueDisplayWBP_C"))
  (UserInterface|Viewport|AddtoViewport _returnvalue 0)
  (bind _returnvalue_2 (UserInterface|CreateWidget "/Game/Blueprints/Widgets/DialogueBoxWBP.DialogueBoxWBP_C" 0 (Utilities|Array|MakeArray "Places, places, everyone! Ready? A one, a two, a one two three fo-") 3.5))
  (Default|AddWidgettoStack _returnvalue _returnvalue_2)
  (return _returnvalue_2))

(fn MusicIdles
  (bind _outactors (Actor|GetAllActorsOfClass "/Game/Blueprints/PennyBP.PennyBP_C"))
  (Components|Animation|PlayAnimation (Variables|/Game/Blueprints/PennyBP.PennyBP_C|GetT-Pose (Utilities|Array|Get(acopy) _outactors)) "/Game/Assets/Animations/Penny_anims/Anim_0_Penny_music_idle.Anim_0_Penny_music_idle" true)
  (bind _outactors_2 (Actor|GetAllActorsOfClass "/Game/Blueprints/TabbieBP.TabbieBP_C"))
  (Components|Animation|PlayAnimation (Variables|/Game/Blueprints/TabbieBP.TabbieBP_C|GetTabbie_tp_fixed (Utilities|Array|Get(acopy) _outactors_2)) "/Game/Assets/Animations/TabbieFix_Anim/Music_idle.Music_idle" true)
  (bind _outactors_3 (Actor|GetAllActorsOfClass "/Game/Blueprints/BunbunBP.BunbunBP_C"))
  (Components|Animation|PlayAnimation (Variables|/Game/Blueprints/BunbunBP.BunbunBP_C|GetBunbun_tp_fixed (Utilities|Array|Get(acopy) _outactors_3)) "/Game/Assets/Animations/BunbunFix_Anim/Idle.Idle" true)
  (bind _outactors_4 (Actor|GetAllActorsOfClass "/Game/Blueprints/TeddyBP.TeddyBP_C"))
  (Components|Animation|PlayAnimation (Variables|/Game/Blueprints/TeddyBP.TeddyBP_C|GetT_Pose (Utilities|Array|Get(acopy) _outactors_4)) "/Game/Assets/Animations/Teddy_Anima/Music_idle.Music_idle" true))