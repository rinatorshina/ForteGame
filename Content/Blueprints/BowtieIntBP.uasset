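; BowtieIntBP is an interactable bowtie pickup for a quest given by Teddy.
; When gazed at, it enables input and marks itself looked at only if SpokeToTeddy is true, blocking interaction before the quest starts.
; On interaction, it sets HasBowtie on the first TeddyBP found in the level, then destroys itself.
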(event EventGazedat
  ;[0.15 0.15 0.15 0.5] Prevents player from interacting with bowtie before quest start
  (if (Variables|Default|GetSpokeToTeddy)
    (Input|EnableInput 0)
    (Variables|Default|SetLookedAt true)
    (else
      (Input|DisableInput 0)
      (Variables|Default|SetLookedAt false))))

(event EventOnInteractedwith
  ;[0.15 0.15 0.15 0.5] Pick up bowtie
  (bind _outactors (Actor|GetAllActorsOfClass "/Game/Blueprints/TeddyBP.TeddyBP_C"))
  (Variables|/Game/Blueprints/TeddyBP.TeddyBP_C|SetHasBowtie (Utilities|Array|Get(acopy) _outactors) true)
  (Actor|DestroyActor))

(fn ConstructionScript
  (|CallParentFunction))