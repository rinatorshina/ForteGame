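; Teddy quest NPC that asks the player to find its missing bowtie, with dialogue shown via PrintString.
; The first request sets SpokeToTeddy on the BowtieIntBP actor.
; With HasBowtie set, interaction calls SwitchState on the StateSwitchManager if its TriggerCount is below one, otherwise completes the quest only in one specific state.
; GiveBowtie swaps visibility between the plain and bowtie-wearing teddy components.
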(event EventOnInteractedwith
  (if (Variables|Default|GetHasBowtie)
    (if (Variables|Default|GetTeddyQuestCompleted)
      (Development|PrintString "Now help others")
      (elif (>= (Variables|/Game/Blueprints/StateSwitchManager.StateSwitchManager_C|GetTriggerCount (Utilities|Array|Get(acopy) (stale EventBeginPlay _outactors))) 1)
        (if (Utilities|Enum|Equal(Enum) (Variables|/Game/Blueprints/StateSwitchManager.StateSwitchManager_C|GetCurrentState (Utilities|Array|Get(acopy) (stale EventBeginPlay _outactors))) "NewEnumerator0")
          (CallFunction|GiveBowtie)
          (Development|PrintString "Yay, thank you!")
          (Variables|Default|SetTeddyQuestCompleted true)
          (else
            (Development|PrintString "Focus")))
        (else
          (Default|SwitchState (Utilities|Array|Get(acopy) (stale EventBeginPlay _outactors))))))
    (elif (Variables|Default|GetTeddyQuestActive)
      (Development|PrintString "Told you to find the bowtie, didn't I?")
      (else
        (Variables|Default|SetTeddyQuestActive true)
        (Development|PrintString "I can't find my bowtie, can you help?")
        (bind _outactors (Actor|GetAllActorsOfClass "/Game/Blueprints/BowtieIntBP.BowtieIntBP_C"))
        (Variables|/Game/Blueprints/BowtieIntBP.BowtieIntBP_C|SetSpokeToTeddy (Utilities|Array|Get(acopy) _outactors) true)))))

(event EventBeginPlay
  ;[0.15 0.15 0.15 0.5] Makes bowtie invisible at the start
  (Rendering|SetVisibility (Variables|Default|GetTeddy_with_tie) false false)
  ;[0.15 0.15 0.15 0.5] Get State Switch Manager
  (bind _outactors (Actor|GetAllActorsOfClass "/Game/Blueprints/StateSwitchManager.StateSwitchManager_C")))

(fn ConstructionScript
  (|CallParentFunction))

(fn GiveBowtie
  (Rendering|SetVisibility (Variables|Default|GetTeddy_with_tie) true false)
  (Rendering|SetVisibility (Variables|Default|GetTeddy1) false false))