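; Bunbun NPC, a stuttering trumpet-playing bunny whose dialogue follows the band quest and ends in a wish confession that sets SolutionAvailable.
; On interaction it checks StateSwitchManager, showing a focus hint outside the required state, otherwise picking a line from its own, Teddy, Penny and Tabbie progress flags.
; Each line function spawns a typewriter dialogue widget and plays Talking.
; The event graph polls TypewriterFinished each tick before returning to Idle.
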(event EventBeginPlay
  (bind _outactors (Actor|GetAllActorsOfClass "/Game/Blueprints/StateSwitchManager.StateSwitchManager_C"))
  (bind _asbp_first_person_character (Utilities|Casting|CastToBP_FirstPersonCharacter (Game|Player|GetPlayerPawn 0)))
  (Variables|Default|SetPlayer _asbp_first_person_character))

(event EventOnInteractedwith
  (if (Utilities|Enum|Equal(Enum) (Variables|/Game/Blueprints/StateSwitchManager.StateSwitchManager_C|GetCurrentState (Utilities|Array|Get(acopy) (stale EventBeginPlay _outactors))) "NewEnumerator0")
    (bind _outactors (Actor|GetAllActorsOfClass "/Game/Blueprints/TeddyBP.TeddyBP_C"))
    (if (Variables|/Game/Blueprints/TeddyBP.TeddyBP_C|GetTeddyQuestCompleted (Utilities|Array|Get(acopy) _outactors))
      (if (Variables|Default|GetSpokenWith)
        (bind _outactors_2 (Actor|GetAllActorsOfClass "/Game/Blueprints/PennyBP.PennyBP_C"))
        (if (Variables|/Game/Blueprints/PennyBP.PennyBP_C|GetSpokeWith (Utilities|Array|Get(acopy) _outactors_2))
          (bind _outactors_3 (Actor|GetAllActorsOfClass "/Game/Blueprints/TabbieBP.TabbieBP_C"))
          (if (Variables|/Game/Blueprints/TabbieBP.TabbieBP_C|GetSpokenTo (Utilities|Array|Get(acopy) _outactors_3))
            (bind _outactors_4 (Actor|GetAllActorsOfClass "/Game/Blueprints/TabbieBP.TabbieBP_C"))
            (if (Variables|/Game/Blueprints/TabbieBP.TabbieBP_C|GetBunbunMentioned (Utilities|Array|Get(acopy) _outactors_4))
              (if (Variables|Default|GetSolutionAvailable)
                (bind _dialogue_box (CallFunction|AfterEveryoneIdle))
                (if (Variables|/Game/Blueprints/Widgets/DialogueBoxWBP.DialogueBoxWBP_C|GetTypewriterFinished _dialogue_box) :!label _label
                  (Components|Animation|PlayAnimation (Variables|Default|GetBunbun_tp_fixed) "/Game/Assets/Animations/BunbunFix_Anim/Idle.Idle" true)
                  (else
                    (Utilities|FlowControl|DelayUntilNextTick)
                    (goto _label)))
                (else
                  (bind _dialogue_box_2 (CallFunction|AfterEveryoneReveal))
                  (if (Variables|/Game/Blueprints/Widgets/DialogueBoxWBP.DialogueBoxWBP_C|GetTypewriterFinished _dialogue_box_2) :!label _label_2
                    (bind _dialogue_box_3 (CallFunction|AfterEveryoneContinued))
                    (if (Variables|/Game/Blueprints/Widgets/DialogueBoxWBP.DialogueBoxWBP_C|GetTypewriterFinished _dialogue_box_3) :!label _label_3
                      (Components|Animation|PlayAnimation (Variables|Default|GetBunbun_tp_fixed) "/Game/Assets/Animations/BunbunFix_Anim/Idle.Idle" true)
                      (Variables|Default|SetSolutionAvailable true)
                      (else
                        (Utilities|FlowControl|DelayUntilNextTick)
                        (goto _label_3)))
                    (else
                      (Utilities|FlowControl|DelayUntilNextTick)
                      (goto _label_2)))))
              (else
                (bind _dialogue_box_4 (CallFunction|YesPennyNoTabbieIdle :!label _label_4))
                (if (Variables|/Game/Blueprints/Widgets/DialogueBoxWBP.DialogueBoxWBP_C|GetTypewriterFinished _dialogue_box_4) :!label _label_5
                  (Components|Animation|PlayAnimation (Variables|Default|GetBunbun_tp_fixed) "/Game/Assets/Animations/BunbunFix_Anim/Idle.Idle" true)
                  (else
                    (Utilities|FlowControl|DelayUntilNextTick)
                    (goto _label_5)))))
            (else
              (goto _label_4)))
          (else
            (bind _outactors_5 (Actor|GetAllActorsOfClass "/Game/Blueprints/TabbieBP.TabbieBP_C"))
            (if (Variables|/Game/Blueprints/TabbieBP.TabbieBP_C|GetSpokenTo (Utilities|Array|Get(acopy) _outactors_5))
              (bind _dialogue_box_5 (CallFunction|NoPennyYesTabbieIdle))
              (if (Variables|/Game/Blueprints/Widgets/DialogueBoxWBP.DialogueBoxWBP_C|GetTypewriterFinished _dialogue_box_5) :!label _label_6
                (Components|Animation|PlayAnimation (Variables|Default|GetBunbun_tp_fixed) "/Game/Assets/Animations/BunbunFix_Anim/Idle.Idle" true)
                (else
                  (Utilities|FlowControl|DelayUntilNextTick)
                  (goto _label_6)))
              (else
                (bind _dialogue_box_6 (CallFunction|BeforeEveryoneIdle))
                (if (Variables|/Game/Blueprints/Widgets/DialogueBoxWBP.DialogueBoxWBP_C|GetTypewriterFinished _dialogue_box_6) :!label _label_7
                  (Components|Animation|PlayAnimation (Variables|Default|GetBunbun_tp_fixed) "/Game/Assets/Animations/BunbunFix_Anim/Idle.Idle" true)
                  (else
                    (Utilities|FlowControl|DelayUntilNextTick)
                    (goto _label_7)))))))
        (else
          (bind _dialogue_box_7 (CallFunction|OpeningDialogue))
          (if (Variables|/Game/Blueprints/Widgets/DialogueBoxWBP.DialogueBoxWBP_C|GetTypewriterFinished _dialogue_box_7) :!label _label_8
            (Components|Animation|PlayAnimation (Variables|Default|GetBunbun_tp_fixed) "/Game/Assets/Animations/BunbunFix_Anim/Idle.Idle" true)
            (Variables|Default|SetSpokenWith true)
            (else
              (Utilities|FlowControl|DelayUntilNextTick)
              (goto _label_8)))))
      (else
        (bind _dialogue_box_8 (CallFunction|BlankIdle))
        (if (Variables|/Game/Blueprints/Widgets/DialogueBoxWBP.DialogueBoxWBP_C|GetTypewriterFinished _dialogue_box_8) :!label _label_9
          (Components|Animation|PlayAnimation (Variables|Default|GetBunbun_tp_fixed) "/Game/Assets/Animations/BunbunFix_Anim/Idle.Idle" true)
          (else
            (Utilities|FlowControl|DelayUntilNextTick)
            (goto _label_9)))))
    (else
      (CallFunction|RealityState))))

(fn ConstructionScript
  (|CallParentFunction))

(fn BlankIdle
  (Components|Animation|PlayAnimation (Variables|Default|GetBunbun_tp_fixed) "/Game/Assets/Animations/BunbunFix_Anim/Talking.Talking" true)
  (Default|HidePrompt (Variables|Default|GetPlayer))
  (bind _returnvalue (UserInterface|CreateWidget "/Game/Blueprints/Widgets/DialogueDisplayWBP.DialogueDisplayWBP_C"))
  (UserInterface|Viewport|AddtoViewport _returnvalue 0)
  (bind _returnvalue_2 (UserInterface|CreateWidget "/Game/Blueprints/Widgets/DialogueBoxWBP.DialogueBoxWBP_C" 0 (Utilities|Array|MakeArray "Oh... H-hey, Sammy... Um, I think Teddy wanted to talk to you...") 3.5))
  (Default|AddWidgettoStack _returnvalue _returnvalue_2)
  (return _returnvalue_2))

(fn OpeningDialogue
  (Components|Animation|PlayAnimation (Variables|Default|GetBunbun_tp_fixed) "/Game/Assets/Animations/BunbunFix_Anim/Talking.Talking" true)
  (Default|HidePrompt (Variables|Default|GetPlayer))
  (bind _returnvalue (UserInterface|CreateWidget "/Game/Blueprints/Widgets/DialogueDisplayWBP.DialogueDisplayWBP_C"))
  (UserInterface|Viewport|AddtoViewport _returnvalue 0)
  (bind _returnvalue_2 (UserInterface|CreateWidget "/Game/Blueprints/Widgets/DialogueBoxWBP.DialogueBoxWBP_C" 0 (Utilities|Array|MakeArray "I-I'm the bun who can't get anything done... I've got one job in th-th-this band: just blow my own trumpet and I can't even do that...") 5.0))
  (Default|AddWidgettoStack _returnvalue _returnvalue_2)
  (return _returnvalue_2))

(fn BeforeEveryoneIdle
  (Components|Animation|PlayAnimation (Variables|Default|GetBunbun_tp_fixed) "/Game/Assets/Animations/BunbunFix_Anim/Talking.Talking" true)
  (Default|HidePrompt (Variables|Default|GetPlayer))
  (bind _returnvalue (UserInterface|CreateWidget "/Game/Blueprints/Widgets/DialogueDisplayWBP.DialogueDisplayWBP_C"))
  (UserInterface|Viewport|AddtoViewport _returnvalue 0)
  (bind _returnvalue_2 (UserInterface|CreateWidget "/Game/Blueprints/Widgets/DialogueBoxWBP.DialogueBoxWBP_C" 0 (Utilities|Array|MakeArray "I don't understand, my wish didn't come true... S-sorry, Sammy, I've spoilt your concert...") 3.5))
  (Default|AddWidgettoStack _returnvalue _returnvalue_2)
  (return _returnvalue_2))

(fn YesPennyNoTabbieIdle
  (Components|Animation|PlayAnimation (Variables|Default|GetBunbun_tp_fixed) "/Game/Assets/Animations/BunbunFix_Anim/Talking.Talking" true)
  (Default|HidePrompt (Variables|Default|GetPlayer))
  (bind _returnvalue (UserInterface|CreateWidget "/Game/Blueprints/Widgets/DialogueDisplayWBP.DialogueDisplayWBP_C"))
  (UserInterface|Viewport|AddtoViewport _returnvalue 0)
  (bind _returnvalue_2 (UserInterface|CreateWidget "/Game/Blueprints/Widgets/DialogueBoxWBP.DialogueBoxWBP_C" 0 (Utilities|Array|MakeArray "Oh, dear... P-Penny seems so upset... If only I could help...") 2.5))
  (Default|AddWidgettoStack _returnvalue _returnvalue_2)
  (return _returnvalue_2))

(fn NoPennyYesTabbieIdle
  (Components|Animation|PlayAnimation (Variables|Default|GetBunbun_tp_fixed) "/Game/Assets/Animations/BunbunFix_Anim/Talking.Talking" true)
  (Default|HidePrompt (Variables|Default|GetPlayer))
  (bind _returnvalue (UserInterface|CreateWidget "/Game/Blueprints/Widgets/DialogueDisplayWBP.DialogueDisplayWBP_C"))
  (UserInterface|Viewport|AddtoViewport _returnvalue 0)
  (bind _returnvalue_2 (UserInterface|CreateWidget "/Game/Blueprints/Widgets/DialogueBoxWBP.DialogueBoxWBP_C" 0 (Utilities|Array|MakeArray "You sh-shouldn't worry about me, Sammy... I don't want to take too much of your time...") 3.5))
  (Default|AddWidgettoStack _returnvalue _returnvalue_2)
  (return _returnvalue_2))

(fn AfterEveryoneReveal
  (Components|Animation|PlayAnimation (Variables|Default|GetBunbun_tp_fixed) "/Game/Assets/Animations/BunbunFix_Anim/Talking.Talking" true)
  (Default|HidePrompt (Variables|Default|GetPlayer))
  (bind _returnvalue (UserInterface|CreateWidget "/Game/Blueprints/Widgets/DialogueDisplayWBP.DialogueDisplayWBP_C"))
  (UserInterface|Viewport|AddtoViewport _returnvalue 0)
  (bind _returnvalue_2 (UserInterface|CreateWidget "/Game/Blueprints/Widgets/DialogueBoxWBP.DialogueBoxWBP_C" 0 (Utilities|Array|MakeArray "Everyone's cross and I don't know why. I made a w-w-wish - I suppose I can tell you now because it hasn't come true..." "I wished the band would all get along, as if we were all one family, and play the perfect concert for you, Sammy.") 4.0))
  (Default|AddWidgettoStack _returnvalue _returnvalue_2)
  (return _returnvalue_2))

(fn AfterEveryoneContinued
  (Components|Animation|PlayAnimation (Variables|Default|GetBunbun_tp_fixed) "/Game/Assets/Animations/BunbunFix_Anim/Talking.Talking" true)
  (Default|HidePrompt (Variables|Default|GetPlayer))
  (bind _returnvalue (UserInterface|CreateWidget "/Game/Blueprints/Widgets/DialogueDisplayWBP.DialogueDisplayWBP_C"))
  (UserInterface|Viewport|AddtoViewport _returnvalue 0)
  (bind _returnvalue_2 (UserInterface|CreateWidget "/Game/Blueprints/Widgets/DialogueBoxWBP.DialogueBoxWBP_C" 0 (Utilities|Array|MakeArray "I f-found a lucky penny on the floor of the fort this morning and I really thought it would work." "I even p-p-put it in my trumpet to make sure my wish was extra loud..." "But that only broke it! Oh, d-dear, is there nothing this bun can do right...") 3.5))
  (Default|AddWidgettoStack _returnvalue _returnvalue_2)
  (return _returnvalue_2))

(fn AfterEveryoneIdle
  (Components|Animation|PlayAnimation (Variables|Default|GetBunbun_tp_fixed) "/Game/Assets/Animations/BunbunFix_Anim/Talking.Talking" true)
  (Default|HidePrompt (Variables|Default|GetPlayer))
  (bind _returnvalue (UserInterface|CreateWidget "/Game/Blueprints/Widgets/DialogueDisplayWBP.DialogueDisplayWBP_C"))
  (UserInterface|Viewport|AddtoViewport _returnvalue 0)
  (bind _returnvalue_2 (UserInterface|CreateWidget "/Game/Blueprints/Widgets/DialogueBoxWBP.DialogueBoxWBP_C" 0 (Utilities|Array|MakeArray "Maybe that was an UN-lucky penny...") 2.5))
  (Default|AddWidgettoStack _returnvalue _returnvalue_2)
  (return _returnvalue_2))

(fn RealityState
  (Default|HidePrompt (Variables|Default|GetPlayer))
  (bind _returnvalue (UserInterface|CreateWidget "/Game/Blueprints/Widgets/DialogueDisplayWBP.DialogueDisplayWBP_C"))
  (UserInterface|Viewport|AddtoViewport _returnvalue 0)
  (bind _returnvalue_2 (UserInterface|CreateWidget "/Game/Blueprints/Widgets/DialogueBoxWBP.DialogueBoxWBP_C" 0 (Utilities|Array|MakeArray "Focus by holding down [Space Bar]") 3.0))
  (Default|AddWidgettoStack _returnvalue _returnvalue_2)
  (return _returnvalue_2))